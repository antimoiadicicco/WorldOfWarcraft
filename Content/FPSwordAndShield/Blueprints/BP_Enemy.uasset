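; BP_Enemy is an AI-driven enemy that damages the player on contact, reports fights to the game mode, and explodes when killed.
; Pawn sensing sets the blackboard TargetActor, cleared after a short retriggerable delay, while Tick writes player distance to Near.
; Tick also polls capsule overlaps, dealing damage and starting the fight when DoesDamage is set, then clearing that flag.
; HP component events update and camera-orient the health bar, and end the fight on death.
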(event OnSeePawn(PawnSensing)
  (params (Pawn :type Pawn%20Object%20Reference))
  (bind _returnvalue (Utilities|Name|MakeLiteralName "TargetActor"))
  (bind _self self)
  (bind _returnvalue_2 (AI|GetAIController _self))
  (bind _returnvalue_3 (AI|GetBlackboard _returnvalue_2))
  (AI|Components|Blackboard|SetValueasObject _returnvalue_3 _returnvalue Pawn)
  (Utilities|FlowControl|RetriggerableDelay 2.0)
  (AI|Components|Blackboard|ClearValue _returnvalue_3 _returnvalue))

(event UpdateHealth(HP_Component)
  (params (Notifaction%20Current%20Health :type Float%20%28double-precision%29))
  (bind _healthbar (Variables|Default|GetHealthBar))
  (Development|PrintString (Utilities|String|ToString(Float) Notifaction%20Current%20Health))
  (bind _ashealth_bar (Utilities|Casting|CastToHealthBar (UserInterface|GetWidget (Variables|Default|GetHealthBar))))
  (Progress|SetPercent (Variables|/Game/FPSwordAndShield/Blueprints/HealthBar.HealthBar_C|GetHealthBar _ashealth_bar) (/ (Variables|Default|GetHealth) 1e+02))
  (Transformation|SetWorldRotation _healthbar (Math|Rotator|FindLookatRotation (Transformation|GetWorldLocation _healthbar) (Transformation|GetWorldLocation (Variables|/Script/Engine.PlayerCameraManager|GetTransformComponent (Game|GetPlayerCameraManager 0)))) false false))

(event Death(HP_Component)
  (Development|PrintString "died")
  (Default|EndFight (.AsFirst%20Person%20Game%20Mode (Utilities|Casting|CastToFirstPersonGameMode (Game|GetGameMode))) self)
  (Audio|PlaySound2D "/Game/Free_Sounds_Pack/wav/Explosion_Medium_2-1.Explosion_Medium_2-1" 1.0 1.0 0.0 0 0)
  (Actor|DestroyActor))

(event Collision|EventActorBeginOverlap
  (params (OtherActor :type Actor%20Object%20Reference)))

(event EventTick
  (params (DeltaSeconds :type Float%20%28single-precision%29))
  (|CallParentFunction DeltaSeconds)
  (Utilities|FlowControl|Sequence
    (:then_0
      (for _array_element (Collision|GetOverlappingActors (Variables|Default|GetCapsule) "/Script/Engine.Actor" :!class /Script/Engine.PrimitiveComponent)
        (bind _asbp_player (Utilities|Casting|CastToBP_Player _array_element))
        (if (Variables|Default|Getdoes%20damage?)
          (Default|StartFight (.AsFirst%20Person%20Game%20Mode (Utilities|Casting|CastToFirstPersonGameMode (Game|GetGameMode))) self)
          (Default|Damage (Variables|/Game/FPSwordAndShield/Blueprints/BP_Character.BP_Character_C|GetHP_Component _asbp_player) (Variables|Default|GetDamage))
          (Variables|Default|Setdoes%20damage? false))))
    (:then_1
      (AI|Components|Blackboard|SetValueasFloat (AI|GetBlackboard (AI|GetAIController self)) (Utilities|Name|MakeLiteralName "Near") (Math|Vector|Distance(Vector) (Transformation|GetActorLocation) (Transformation|GetActorLocation (Game|Player|GetPlayerPawn 0)))))))

(event EventBeginPlay)

(fn ConstructionScript
  (|CallParentFunction))