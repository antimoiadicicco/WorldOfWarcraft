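; HP_Component is a health component that tracks its owner's current health, starting at maximum on BeginPlay.
; Its Damage function ignores hits while IsBlocking is set; otherwise it subtracts the amount from current health and reports it to FirstPersonGameMode.
; It then broadcasts the new value through the UpdateHealth dispatcher and fires Death when health reaches zero or below.
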(event EventBeginPlay
  (Variables|Default|SetCurrent%20Health (Variables|Default|GetMaximumHealth)))

(fn Damage
  (params (Damage :type Float%20%28double-precision%29))
  (if (not (Variables|Default|GetIs%20Blocking?))
    (Variables|Default|SetCurrent%20Health (- (Variables|Default|GetCurrent%20Health) Damage))
    (Default|AddDamageTaken (.AsFirst%20Person%20Game%20Mode (Utilities|Casting|CastToFirstPersonGameMode (Game|GetGameMode))) Damage self)
    (Default|CallUpdateHealth (Variables|Default|GetCurrent%20Health))
    (if (<= (Variables|Default|GetCurrent%20Health) 0.0)
      (Default|CallDeath))))