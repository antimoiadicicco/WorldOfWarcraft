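; Player Blueprint for a first-person sword-and-shield game, handling health feedback, death and damage dealt to enemies.
; HP_Component events print remaining health to screen and open DemoMap on death.
; Tick polls the Capsule's overlapping actors and damages a BP_Enemy through its HPComponent while DoesDamage is set, then clears the flag so only one hit lands.
; Nothing in this file re-arms that flag.
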(event UpdateHealth(HP_Component)
  (params (Notifaction%20Current%20Health :type Float%20%28double-precision%29))
  (Development|PrintString "Vita rimanente:")
  (Development|PrintString (Utilities|String|ToString(Float) Notifaction%20Current%20Health)))

(event Death(HP_Component)
  (Development|PrintString "Mortoooooo")
  (Game|OpenLevel(byObjectReference) "/Game/FPSwordAndShield/Maps/DemoMap.DemoMap"))

(event EventBeginPlay
  (|CallParentFunction) ; This node is disabled and will not be called.\nDrag off pins to build functionality.
)

(event Collision|EventActorBeginOverlap
  (params (OtherActor :type Actor%20Object%20Reference)))

(event EventTick
  (params (DeltaSeconds :type Float%20%28single-precision%29))
  (for _array_element (Collision|GetOverlappingActors (Variables|Default|GetCapsule) "/Script/Engine.Actor" :!class /Script/Engine.PrimitiveComponent)
    (bind _asbp_enemy (Utilities|Casting|CastToBP_Enemy _array_element))
    (if (Variables|Default|Getdoes%20damage?)
      (Default|Damage (Variables|/Game/FPSwordAndShield/Blueprints/BP_Character.BP_Character_C|GetHP_Component _asbp_enemy) (Variables|Default|GetDamage))
      (Variables|Default|Setdoes%20damage? false))))

(fn ConstructionScript
  (|CallParentFunction))