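; BlockSpot is an anim notify state that marks the window in an animation during which a character is blocking.
; On begin it casts the mesh owner to BP_Character and sets IsBlocking to true on its HPComponent.
; On end it sets the same flag back to false, so the length of the notify defines the block duration.
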(fn ReceivedNotifyBegin
  (params (MeshComp :type Skeletal%20Mesh%20Component%20Object%20Reference) (Animation :type Anim%20Sequence%20Base%20Object%20Reference) (TotalDuration :type Float%20%28single-precision%29) (EventReference :type Anim%20Notify%20Event%20Reference%20Structure%20%28by%20ref%29))
  (Variables|/Game/FPSwordAndShield/Blueprints/HP_Component.HP_Component_C|SetIs%20Blocking? (Variables|/Game/FPSwordAndShield/Blueprints/BP_Character.BP_Character_C|GetHP_Component (.AsBP%20Player (Utilities|Casting|CastToBP_Character (Components|GetOwner MeshComp)))) true)
  (return false))

(fn ReceivedNotifyEnd
  (params (MeshComp :type Skeletal%20Mesh%20Component%20Object%20Reference) (Animation :type Anim%20Sequence%20Base%20Object%20Reference) (EventReference :type Anim%20Notify%20Event%20Reference%20Structure%20%28by%20ref%29))
  (Variables|/Game/FPSwordAndShield/Blueprints/HP_Component.HP_Component_C|SetIs%20Blocking? (Variables|/Game/FPSwordAndShield/Blueprints/BP_Character.BP_Character_C|GetHP_Component (.AsBP%20Player (Utilities|Casting|CastToBP_Character (Components|GetOwner MeshComp)))) false)
  (return false))