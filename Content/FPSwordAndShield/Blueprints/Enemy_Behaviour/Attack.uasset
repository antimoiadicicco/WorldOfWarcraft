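; Behavior tree task that makes a BP_Enemy play its melee attack animation.
; On execute, it checks that the blackboard "Near" value is within a fixed range and that the player's HP component shows health above zero.
; It then plays the attack montage on the enemy's Mesh2P and finishes successfully only when the montage completes.
; Failed checks, a failed enemy cast or an interrupted montage never call FinishExecute.
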(event EventReceiveExecuteAI
  (params (OwnerController :type AI%20Controller%20Object%20Reference) (ControlledPawn :type Pawn%20Object%20Reference))
  (if (and (<= (Class|BlackboardComponent|GetValueasFloat (AI|GetBlackboard (AI|GetAIController ControlledPawn)) (Utilities|Name|MakeLiteralName "Near")) 3e+02) (> (Variables|/Game/FPSwordAndShield/Blueprints/HP_Component.HP_Component_C|GetCurrent%20Health (Variables|/Game/FPSwordAndShield/Blueprints/BP_Character.BP_Character_C|GetHP_Component (.AsBP%20Player (Utilities|Casting|CastToBP_Player (Game|Player|GetPlayerPawn 0))))) 0.0))
    (bind _asbp_enemy (Utilities|Casting|CastToBP_Enemy ControlledPawn))
    (Animation|Montage|PlayMontage (Variables|/Game/FPSwordAndShield/Blueprints/BP_Character.BP_Character_C|GetMesh2P _asbp_enemy) "/Game/FPSwordAndShield/Animations/AttackMontage.AttackMontage" 1.0 0.0 "None" false
      (:OnCompleted
        (AI|BehaviorTree|FinishExecute true)))))