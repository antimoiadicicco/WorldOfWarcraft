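; BP_Lion is an enemy that chases the first player's pawn.
; From BeginPlay, an AI MoveTo loop retries after a short delay on success or failure.
; A parallel timed loop toggles a Rest flag that this graph never reads, and a third branch ends in an unconnected delay.
; The health component's Death event only prints a message.
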(event Death(AC_HealthComponent)
  (Development|PrintString "Died"))

(event EventBeginPlay
  (|CallParentFunction)
  (Utilities|FlowControl|Sequence
    (:then_0
      (AI|AIMoveTo self "0, 0, 0" (Game|Player|GetPlayerPawn 0) 5.0 false :!label _label
        (:OnSuccess
          _)
        (:OnFail
          _))
      (Utilities|FlowControl|Delay 2.0)
      (goto _label))
    (:then_1
      (Utilities|FlowControl|Delay 5.0 :!label _label_2)
      (Variables|Default|SetRest true)
      (Utilities|FlowControl|Delay 5.0)
      (Variables|Default|SetRest false)
      (goto _label_2))
    (:then_2
      (Utilities|FlowControl|Delay 15.0))))

(event Collision|EventActorBeginOverlap
  (params (OtherActor :type Actor%20Object%20Reference))
  (|CallParentFunction OtherActor) ; This node is disabled and will not be called.\nDrag off pins to build functionality.
)

(event EventTick
  (params (DeltaSeconds :type Float%20%28single-precision%29))
  (|CallParentFunction DeltaSeconds) ; This node is disabled and will not be called.\nDrag off pins to build functionality.
)

(fn ConstructionScript
  (|CallParentFunction))